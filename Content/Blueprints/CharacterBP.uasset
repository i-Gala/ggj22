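; Player character that moves on world X/Y axes, throws an anchor and pulls itself to it.
; ThrowPull either spawns AnchorBP, with gravity delayed by TimeInAir, or pulls once the anchor reports sticking to the floor.
; The pull is a timeline lerp in X/Y that destroys the anchor and re-enables throwing.
; ThrowUp alone sets control rotation, ThrowRight is empty, and construction tints the Cone with AnchorColor.
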(event `self.ReceiveBeginPlay`)

(event `InputAxis|MoveUp`
  (params (AxisValue :type "Float (single-precision)"))
  ;[1 1 1] Movement
  (`self.AddMovementInput` (1.0 0.0 0.0) AxisValue))

(event `InputAxis|MoveRight`
  (params (AxisValue :type "Float (single-precision)"))
  ;[1 1 1] Movement
  (`self.AddMovementInput` (0.0 1.0 0.0) AxisValue))

(event `InputAxis|ThrowUp`
  (params (AxisValue :type "Float (single-precision)"))
  (bind _returnvalue (`KismetMathLibrary.MakeVector` AxisValue (stale `InputAxis|ThrowRight` AxisValue)))
  (if (> (`KismetMathLibrary.VSize` _returnvalue) 0.25)
    ;[1 1 1] press stick
    (`Controller.SetControlRotation` (`GameplayStatics.GetPlayerController` 0) (`KismetMathLibrary.Conv_VectorToRotator` _returnvalue))
    ;[1 1 1] release stick
    (if (not (> (`KismetMathLibrary.VSize` _returnvalue) 0.25))
      (`self.Throw`))))

(event `InputAxis|ThrowRight`
  (params (AxisValue :type "Float (single-precision)")))

(event `InputAction|ThrowPull`
  (params (Key :type "Key Structure"))
  (:`Pressed`
    (if (`self.CanThrow`)
      (`self.Throw`)
      (elif (`self.CanPull`)
        (`self.Pull`)))))

(event `Throw`
  (bind _anchorarrow (`self.AnchorArrow`))
  (bind _anchor (`self.Anchor`))
  (bind _projectilemovement (`/Game/Blueprints/AnchorBP.ProjectileMovement` _anchor))
  (if (`self.CanThrow`)
    (set `self.CanThrow` false)
    (`SceneComponent.SetHiddenInGame` (`self.Cone`) true false)
    (bind _returnvalue (`|SpawnActorFromClass` "/Game/Blueprints/AnchorBP.AnchorBP_C" (`KismetMathLibrary.MakeTransform` (`SceneComponent.K2_GetComponentLocation` _anchorarrow) (`SceneComponent.K2_GetComponentRotation` _anchorarrow)) "AdjustIfPossibleButAlwaysSpawn" "OverrideRootScale" self self))
    (set `self.Anchor` _returnvalue)
    (add `/Game/Blueprints/AnchorBP.StuckOnFloor` _anchor (delegate `AnchorStucked`))
    (set `ProjectileMovementComponent.ProjectileGravityScale` 0.0 _projectilemovement)
    (`KismetSystemLibrary.Delay` (`self.TimeInAir`))
    (set `ProjectileMovementComponent.ProjectileGravityScale` 1.0 _projectilemovement)))

(event `AnchorStucked`
  (set `self.CanPull` true))

(event `Pull`
  (bind (_returnvalue_x _returnvalue_y _returnvalue_z) (`KismetMathLibrary.BreakVector` (`self.K2_GetActorLocation` self)))
  (bind (_returnvalue_x_2 _returnvalue_y_2 _returnvalue_z_2) (`KismetMathLibrary.BreakVector` (`self.K2_GetActorLocation` (`self.Anchor`))))
  (set `self.CanPull` false)
  (bind (_direction _moveactor) (`Timeline|Timeline_1` :!via `PlayFromStart`)
    (:`Update`
      (bind (_returnvalue_x_3 _returnvalue_y_3) (`KismetMathLibrary.BreakVector` (`KismetMathLibrary.VLerp` (`KismetMathLibrary.MakeVector` _returnvalue_x _returnvalue_y _returnvalue_z) (`KismetMathLibrary.MakeVector` _returnvalue_x_2 _returnvalue_y_2 _returnvalue_z_2) _moveactor)))
      (`self.K2_SetActorLocation` (`KismetMathLibrary.MakeVector` _returnvalue_x_3 _returnvalue_y_3 _returnvalue_z)))
    (:`Finished`
      (`self.K2_DestroyActor` (`self.Anchor`))
      (`self.EnableInput` null)
      (`SceneComponent.SetHiddenInGame` (`self.Cone`) false false)
      (set `self.CanThrow` true))))

(fn `UserConstructionScript`
  (bind _returnvalue (`PrimitiveComponent.CreateDynamicMaterialInstance` (`self.Cone`) 0 "/Game/Materials/BaseColor.BaseColor" "None"))
  (`MaterialInstanceDynamic.SetVectorParameterValue` _returnvalue "BaseColor" (`self.AnchorColor`)))