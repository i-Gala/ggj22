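; AnchorBP is a projectile anchor that sticks to the floor when it lands.
; When its sphere overlaps a FloorBP, it zeroes projectile movement and gravity, holds its position, snaps to a fixed rotation and calls the StuckOnFloor dispatcher.
; The construction script gives the cone a dynamic material tinted by the Color variable.
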(event `self.Sphere.OnComponentBeginOverlap`
  (params (OverlappedComponent :type "PrimitiveComponent Object Reference") (OtherActor :type "Actor Object Reference") (OtherComp :type "PrimitiveComponent Object Reference") (OtherBodyIndex :type Integer) (bFromSweep :type Boolean) (SweepResult :type "HitResult Structure (by ref)"))
  (bind _projectilemovement (`self.ProjectileMovement`))
  (cast `/Game/Blueprints/FloorBP` OtherActor)
  (set `ProjectileMovementComponent.InitialSpeed` 0.0 _projectilemovement)
  (set `ProjectileMovementComponent.ProjectileGravityScale` 0.0 _projectilemovement)
  (set `MovementComponent.Velocity` (0.0 0.0 0.0) _projectilemovement)
  (`self.K2_SetActorLocation` (`self.K2_GetActorLocation`))
  (`self.K2_SetActorRotation` (struct :`Pitch` -90.0 :`Roll` -180.0))
  (`self.StuckOnFloor`))

(fn `UserConstructionScript`
  (bind _returnvalue (`PrimitiveComponent.CreateDynamicMaterialInstance` (`self.Cone`) 0 null "None"))
  (`MaterialInstanceDynamic.SetVectorParameterValue` _returnvalue "BaseColor" (`self.Color`)))